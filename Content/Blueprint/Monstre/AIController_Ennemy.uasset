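; AI controller for an enemy monster that runs the BT_Enemy behavior tree on begin play.
; AI perception updates write a sensed BP_Player to the PlayerRef blackboard key.
; When the player is no longer sensed, it clears PlayerRef and stores the stimulus location as LastKnowPlayerLoc.
; A ResetPlayerRef event also clears the reference, and an unconnected comparison is a placeholder for future health logic.
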(event OnTargetPerceptionUpdated(AIPerception)
  (params (Actor :type Actor%20Object%20Reference) (Stimulus :type AI%20Stimulus%20Structure))
  (bind _asbp_player (Utilities|Casting|CastToBP_Player Actor))
  (if (.bsuccessfullysensed Stimulus)
    (AI|Components|Blackboard|SetValueasObject (AI|GetBlackboard _asbp_player) (Utilities|String|StringToName "PlayerRef") _asbp_player)
    (else
      (AI|Components|Blackboard|ClearValue (AI|GetBlackboard 0) (Utilities|String|StringToName "PlayerRef"))
      (AI|Components|Blackboard|SetValueasVector (AI|GetBlackboard 0) (Utilities|String|StringToName "LastKnowPlayerLoc") (.stimuluslocation Stimulus)))))

(event Custom|ResetPlayerRef
  (AI|Components|Blackboard|ClearValue (AI|GetBlackboard 0) (Utilities|String|StringToName "PlayerRef")))

(event EventBeginPlay
  (AI|RunBehaviorTree "/Game/Blueprint/Monstre/BT_Enemy.BT_Enemy"))

(event EventTick
  (params (DeltaSeconds :type Float%20%28single-precision%29)))

(fn ConstructionScript)