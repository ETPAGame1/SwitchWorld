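; First-person player character Blueprint with Enhanced Input movement, look, jump, interaction, and toggleable flashlight and scanner.
; IA_Switch alternates the LightLevel and DarkLevel streamed levels with blocking loads; BeginPlay fires the same FlipFlop, starting in light.
; Interaction sphere-traces from the camera and messages the first BPI_Interact hit, leaving persistent debug drawing.
; Flashlight and scanner flip visibility through server-named events that call client-named ones.
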(event Custom|Toggle%20light%20on%20client
  (params (on? :type Boolean))
  ;[1 1 1] Flashlight
  (Rendering|SetVisibility (Variables|Default|Getflashlight) on? false))

(event Custom|Toggle%20light%20on%20server
  (params (on? :type Boolean))
  ;[1 1 1] Flashlight
  (CallFunction|ToggleLightonClient on?))

(event Custom|Toggle%20scan%20on%20client
  (params (On? :type Boolean))
  ;[1 1 1] Scanner
  (Rendering|SetVisibility (Variables|Default|Getscanner) On? false))

(event Custom|toggle%20scan%20on%20server
  (params (On? :type Boolean))
  ;[1 1 1] Scanner
  (CallFunction|ToggleScanonClient On?))

(event Input|EnhancedActionEvents|EnhancedInputActionIA_Moove
  (params (ActionValue :type Vector%202D%20Structure) (ElapsedSeconds :type Float%20%28single-precision%29) (TriggeredSeconds :type Float%20%28single-precision%29))
  ;[0.6765 1 0.1936] Système de déplacement FPS
  (Pawn|Input|AddMovementInput (Math|Vector|Normalize (+ (* (.x ActionValue) (Transformation|GetActorForwardVector)) (* (Transformation|GetActorRightVector) (.y ActionValue)))) 1.0 false))

(event Input|EnhancedActionEvents|EnhancedInputActionIA_Look
  (params (ActionValue :type Vector%202D%20Structure) (ElapsedSeconds :type Float%20%28single-precision%29) (TriggeredSeconds :type Float%20%28single-precision%29))
  ;[0.6765 1 0.1936] Système de déplacement FPS
  (Pawn|Input|AddControllerPitchInput (.y ActionValue))
  (Pawn|Input|AddControllerYawInput (.x ActionValue)))

(event Input|EnhancedActionEvents|EnhancedInputActionIA_Interact
  (params (ActionValue :type Boolean) (ElapsedSeconds :type Float%20%28single-precision%29) (TriggeredSeconds :type Float%20%28single-precision%29))
  (bind _camera (Variables|Default|GetCamera))
  (bind _returnvalue (Transformation|GetWorldLocation _camera))
  ;[1 1 1] Interaction/raycast
  (bind _outhits (Collision|MultiSphereTraceByChannel _returnvalue (+ (* (Math|Vector|GetForwardVector _camera) (Variables|Default|Getdistance)) _returnvalue) 1e+01 "TraceTypeQuery1" false 0 "Persistent"))
  (bind _array_element (Utilities|Array|ForEachLoopwithBreak _outhits :!label _label)
    (:LoopBody
      (if (Utilities|DoesObjectImplementInterface (.hitactor _array_element) "/Game/Blueprint/Player/BPI_Interact.BPI_Interact_C")
        (Class|BPIInteract|Interact(Message) (.hitactor _array_element))
        (goto _label Break)))))

(event Input|EnhancedActionEvents|EnhancedInputActionIA_Switch
  (params (ActionValue :type Boolean) (ElapsedSeconds :type Float%20%28single-precision%29) (TriggeredSeconds :type Float%20%28single-precision%29))
  ;[0.333 0.9801 1] StreamingLevel
  (Utilities|FlowControl|FlipFlop
    (:A
      (Class|GameplayStatics|LoadStreamLevelbySoftObjectPtr "/Game/LevelStreaming/LightLevel.LightLevel" true true)
      (Class|GameplayStatics|UnloadStreamLevelbySoftObjectPtr "/Game/LevelStreaming/DarkLevel.DarkLevel" true))
    (:B
      (Class|GameplayStatics|LoadStreamLevelbySoftObjectPtr "/Game/LevelStreaming/DarkLevel.DarkLevel" true true)
      (Class|GameplayStatics|UnloadStreamLevelbySoftObjectPtr "/Game/LevelStreaming/LightLevel.LightLevel" true))))

(event Input|EnhancedActionEvents|EnhancedInputActionIA_Jump
  (params (ActionValue :type Vector :default "0, 0, 0") (ElapsedSeconds :type Float%20%28single-precision%29) (TriggeredSeconds :type Float%20%28single-precision%29))
  ;[0.6765 1 0.1936] Système de déplacement FPS
  (Character|Jump))

(event Collision|EventActorBeginOverlap
  (params (OtherActor :type Actor%20Object%20Reference)))

(event EventTick
  (params (DeltaSeconds :type Float%20%28single-precision%29)))

(event EventPossessed
  (params (NewController :type Controller%20Object%20Reference))
  ;[0.6765 1 0.1936] Système de déplacement FPS
  (Input|AddMappingContext (PlayerController|LocalPlayerSubsystems|GetEnhancedInputLocalPlayerSubsystem (Game|GetPlayerController 0)) "/Game/Blueprint/Input/IMC_FirstPersonInput.IMC_FirstPersonInput" 0))

(event EventBeginPlay
  ;[0.333 0.9801 1] StreamingLevel
  (Utilities|FlowControl|FlipFlop
    (:A
      (Class|GameplayStatics|LoadStreamLevelbySoftObjectPtr "/Game/LevelStreaming/LightLevel.LightLevel" true true)
      (Class|GameplayStatics|UnloadStreamLevelbySoftObjectPtr "/Game/LevelStreaming/DarkLevel.DarkLevel" true))
    (:B
      (Class|GameplayStatics|LoadStreamLevelbySoftObjectPtr "/Game/LevelStreaming/DarkLevel.DarkLevel" true true)
      (Class|GameplayStatics|UnloadStreamLevelbySoftObjectPtr "/Game/LevelStreaming/LightLevel.LightLevel" true))))

(event Input|ActionEvents|InputActionflashlight
  (params (Key :type Key%20Structure :default "None"))
  ;[1 1 1] Flashlight
  (:Pressed
    (Utilities|FlowControl|FlipFlop
      (:A
        (CallFunction|ToggleLightonServer true))
      (:B
        (CallFunction|ToggleLightonServer false)))))

(event Input|ActionEvents|InputActionScanner
  (params (Key :type Key%20Structure :default "None"))
  ;[1 1 1] Scanner
  (:Pressed
    (Utilities|FlowControl|FlipFlop
      (:A
        (CallFunction|ToggleScanonServer true))
      (:B
        (CallFunction|ToggleScanonServer false)))))

(fn ConstructionScript)